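; Haptic hit box that, on a RayHit event, plays a short haptic dot on its assigned device position near where the box was struck.
; RayHit passes the hit box component and location to ProjectToPoint, then submits the resulting dot to the HapticManager.
; The projection maps the box-local Y/Z offset onto a per-device grid of motor columns and rows, with separate index handling for the head.
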(event `/HapticsManager/Blueprints/DummyInterface.RayHit`
  (params (Hit :type "HitResult Structure"))
  (bind (_bblockinghit _binitialoverlap _time _distance _location _impactpoint _normal _impactnormal _physmat _hitactor _hitcomponent) (`GameplayStatics.BreakHitResult` Hit))
  ;[1 1 1] Submit haptic feedback of the closest dot to where the collider was hit.
  (bind _asbox_collision (cast `BoxComponent` _hitcomponent))
  (`HapticManagerComponent.SubmitDots` (`self.HapticManager`) "HitDevice" (`self.DevicePosition`) (`|MakeArray` (`self.ProjectToPoint` _asbox_collision _location)) 200))

(fn `UserConstructionScript`)