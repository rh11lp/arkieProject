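; HapticManager_BP is a haptics manager that wires up on-screen dot visualisation for tactsuit devices.
; It passes dot references for sleeves, head, front and back vest, gloves, shoes and racket to SetTactSuit.
; The same call runs in both the Construction Script and BeginPlay, so the references are set on construction and again when play starts.
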(event `self.ReceiveBeginPlay`
  ;[1 1 1] Set the references of the tactsuit dots in the UI for visualisation.
  (`self.SetTactSuit` (`self.TactosyLDots`) (`self.TactosyRDots`) (`self.TactalDots`) (`self.TactotFDots`) (`self.TactotBDots`) (`self.TactGloveLDots`) (`self.TactGloveRDots`) (`self.TactShoesLDots`) (`self.TactShoesRDots`) (`self.Racket`)))

(fn `UserConstructionScript`
  ;[1 1 1] Set the tactsuit dots in the UI for visualisation.
  (`self.SetTactSuit` (`self.TactosyLDots`) (`self.TactosyRDots`) (`self.TactalDots`) (`self.TactotFDots`) (`self.TactotBDots`) (`self.TactGloveLDots`) (`self.TactGloveRDots`) (`self.TactShoesLDots`) (`self.TactShoesRDots`) (`self.Racket`)))